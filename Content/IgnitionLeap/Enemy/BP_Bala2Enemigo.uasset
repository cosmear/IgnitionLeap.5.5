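; Enemy rocket projectile that explodes on hit, or when its overlap sphere touches the player character.
; Both triggers share one explosion chain that applies radial damage and spawns BP_RocketJump, which the comments tie to rocket-jump impulse, plus a particle actor.
; The chain then pushes the hit component along the projectile's velocity, plays an explosion sound and destroys the projectile.
; A separate physics-checked impulse branch is left unconnected.
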(event OnComponentBeginOverlap(Sphere1)
  (params (OverlappedComponent :type Primitive%20Component%20Object%20Reference) (OtherActor :type Actor%20Object%20Reference) (OtherComp :type Primitive%20Component%20Object%20Reference) (OtherBodyIndex :type Integer) (bFromSweep :type Boolean) (SweepResult :type Hit%20Result%20Structure%20%28by%20ref%29))
  (if (== OtherActor (Game|GetPlayerCharacter 0))
    ;[1 1 1] MECHANIC: Rocket
    ;;[0.05035 0.05035 0.05035] Add impulse for the Rocket jump
    (Game|Damage|ApplyRadialDamage (Variables|Default|GetDaño) (Transformation|GetActorLocation) 3e+02 0 0 self 0 false "ECC_Visibility")
    (Game|SpawnActorfromClass "/Game/IgnitionLeap/Blueprints/BP_RocketJump.BP_RocketJump_C" (Math|Transform|MakeTransform (stale Collision|EventHit HitLocation)) "Undefined" "MultiplyWithRoot" 0 0)
    ;;[1 1 1] Add Partcles and sounds to the end of projectiles
    (Game|SpawnActorfromClass "/Game/Realistic_Starter_VFX_Pack_Vol2/Blueprints/Spawn_Particle.Spawn_Particle_C" (Math|Transform|MakeTransform (stale Collision|EventHit HitLocation)) "Undefined" "MultiplyWithRoot" 0 0)
    (Physics|AddImpulseatLocation (stale Collision|EventHit OtherComp) (* (Transformation|GetVelocity) 8e+02) (Transformation|GetActorLocation) "None")
    (Audio|PlaySoundatLocation "/Game/IgnitionLeap/Audio/SC_Explosion.SC_Explosion" "0, 0, 0" "0, 0, 0" 1.0 1.0 0.0 0 0 0 0)
    (Actor|DestroyActor)))

(event Collision|EventHit
  (params (MyComp :type Primitive%20Component%20Object%20Reference) (Other :type Actor%20Object%20Reference) (OtherComp :type Primitive%20Component%20Object%20Reference) (bSelfMoved :type Boolean) (HitLocation :type Vector :default "0, 0, 0") (HitNormal :type Vector :default "0, 0, 0") (NormalImpulse :type Vector :default "0, 0, 0") (Hit :type Hit%20Result%20Structure%20%28by%20ref%29))
  (bind _returnvalue (Math|Transform|MakeTransform HitLocation))
  ;[1 1 1] MECHANIC: Rocket
  ;;[0.05035 0.05035 0.05035] Add impulse for the Rocket jump
  (Game|Damage|ApplyRadialDamage (Variables|Default|GetDaño) (Transformation|GetActorLocation) 3e+02 0 0 self 0 false "ECC_Visibility")
  (Game|SpawnActorfromClass "/Game/IgnitionLeap/Blueprints/BP_RocketJump.BP_RocketJump_C" _returnvalue "Undefined" "MultiplyWithRoot" 0 0)
  ;;[1 1 1] Add Partcles and sounds to the end of projectiles
  (Game|SpawnActorfromClass "/Game/Realistic_Starter_VFX_Pack_Vol2/Blueprints/Spawn_Particle.Spawn_Particle_C" _returnvalue "Undefined" "MultiplyWithRoot" 0 0)
  (Physics|AddImpulseatLocation OtherComp (* (Transformation|GetVelocity) 8e+02) (Transformation|GetActorLocation) "None")
  (Audio|PlaySoundatLocation "/Game/IgnitionLeap/Audio/SC_Explosion.SC_Explosion" "0, 0, 0" "0, 0, 0" 1.0 1.0 0.0 0 0 0 0)
  (Actor|DestroyActor))

(fn ConstructionScript)