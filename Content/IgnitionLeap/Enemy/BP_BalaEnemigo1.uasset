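; BP_BalaEnemigo1 is an enemy bullet that damages the player on contact.
; When Sphere1 overlaps the player character, its DañoaPJ event applies Daño damage with the bullet as causer and destroys the actor.
; An explosion sound then plays at the player's location.
; Overlaps with any other actor are ignored, and the graphs contain no movement logic.
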(event OnComponentBeginOverlap(Sphere1)
  (params (OverlappedComponent :type Primitive%20Component%20Object%20Reference) (OtherActor :type Actor%20Object%20Reference) (OtherComp :type Primitive%20Component%20Object%20Reference) (OtherBodyIndex :type Integer) (bFromSweep :type Boolean) (SweepResult :type Hit%20Result%20Structure%20%28by%20ref%29))
  (if (== OtherActor (Game|GetPlayerCharacter 0))
    (CallFunction|DañoaPJ)
    (Audio|SpawnSoundatLocation "/Game/StarterContent/Audio/Explosion02.Explosion02" (Transformation|GetActorLocation OtherActor) "0, 0, 0" 1.0 1.0 0.0 0 0)))

(event Custom|DañoaPJ
  (Game|Damage|ApplyDamage (Game|GetPlayerCharacter 0) (Variables|Default|GetDaño) 0 self)
  (Actor|DestroyActor))

(fn ConstructionScript)